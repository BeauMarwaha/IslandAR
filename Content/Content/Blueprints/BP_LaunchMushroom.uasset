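; BP_LaunchMushroom is a bounce pad that launches the CH_Birbman player along the mushroom's up vector.
; On BeginPlay it caches the first CH_Birbman in the level as the player.
; Any BoingCollider overlap launches that cached player by LaunchPower, overriding only Z velocity, and plays a one-shot bounce animation on the mushroom.
; The overlap does not check which actor entered.
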(event OnComponentBeginOverlap(BoingCollider)
  (params (OverlappedComponent :type Primitive%20Component%20Object%20Reference) (OtherActor :type Actor%20Object%20Reference) (OtherComp :type Primitive%20Component%20Object%20Reference) (OtherBodyIndex :type Integer) (bFromSweep :type Boolean) (SweepResult :type Hit%20Result%20Structure%20%28by%20ref%29))
  (Character|LaunchCharacter (Variables|Default|GetPlayer) (* (Transformation|GetActorUpVector) (Variables|Default|GetLaunchPower)) false true)
  (Components|Animation|PlayAnimation (Variables|Default|GetMushroom) "/Game/Content/Animations/A_BounceMushroom_Bounce.A_BounceMushroom_Bounce" false))

(event OnComponentHit(BoingCollider)
  (params (HitComponent :type Primitive%20Component%20Object%20Reference) (OtherActor :type Actor%20Object%20Reference) (OtherComp :type Primitive%20Component%20Object%20Reference) (NormalImpulse :type Vector :default "0, 0, 0") (Hit :type Hit%20Result%20Structure%20%28by%20ref%29)))

(event EventTick
  (params (DeltaSeconds :type Float%20%28single-precision%29)))

(event EventBeginPlay
  (bind _outactors (Actor|GetAllActorsOfClass "/Game/Content/Blueprints/CH_Birbman.CH_Birbman_C"))
  (Variables|Default|SetPlayer (Utilities|Array|Get(acopy) _outactors)))

(fn ConstructionScript)