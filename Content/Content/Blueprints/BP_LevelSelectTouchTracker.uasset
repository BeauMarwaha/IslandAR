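; BP_LevelSelectTouchTracker turns horizontal touch swipes into world changes on the level select.
; Press stores the first finger's screen position, and Release compares it with the end position.
; Movement beyond a small distance threshold counts as a swipe, and the dominant axis sets its direction.
; Left swipes call PreviousWorld and right swipes NextWorld on LevelSelect, while taps and vertical swipes do nothing.
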(fn ConstructionScript)

(fn Press
  (bind _returnvalue (Game|GetPlayerController 0))
  (bind (_locationx _locationy) (Class|PlayerController|GetInputTouchState _returnvalue "Touch1"))
  (Variables|Default|SetStartPosition (Math|Vector2D|MakeVector2D _locationx _locationy))
  (Variables|Default|SetIsPressed true))

(fn Release
  (bind _returnvalue (Game|GetPlayerController 0))
  (bind _levelselect (Variables|Default|GetLevelSelect))
  (bind (_locationx _locationy) (Class|PlayerController|GetInputTouchState _returnvalue "Touch1"))
  (bind _returnvalue_2 (Utilities|IsValid _levelselect))
  (if (Variables|Default|GetIsPressed)
    (Variables|Default|SetIsPressed false)
    (Variables|Default|SetEndPosition (Math|Vector2D|MakeVector2D _locationx _locationy))
    ;[1 1 1] Is it a swipe (true) or a touch (false)
    (if (> (Math|Vector2D|Vector2DLength (- (Variables|Default|GetStartPosition) (Variables|Default|GetEndPosition))) 33.0)
      ;[1 1 1] Are we swiping up/down (false) or left/right (true)
      (if (> (Math|Float|Absolute(Float) (.X (Math|Vector2D|BreakVector2D (- (Variables|Default|GetStartPosition) (Variables|Default|GetEndPosition))))) (Math|Float|Absolute(Float) (.Y (Math|Vector2D|BreakVector2D (- (Variables|Default|GetStartPosition) (Variables|Default|GetEndPosition))))))
        ;[1 1 1] Are we swiping left (true) or right (false)
        (if (> (.X (Math|Vector2D|BreakVector2D (- (Variables|Default|GetStartPosition) (Variables|Default|GetEndPosition)))) 0.0)
          ;[1 1 1] Change the current world in level select based on the swipe direction
          (if _returnvalue_2
            (Default|PreviousWorld _levelselect))
          (elif _returnvalue_2
            (Default|NextWorld _levelselect)))))))