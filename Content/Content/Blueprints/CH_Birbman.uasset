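; Birbman character Blueprint that spawns its default controller on BeginPlay and provides movement and jump functions, with no input bindings in the graph.
; Forward and right functions move along fixed world X and Y axes, and forward input also adds controller yaw.
; JumpStart calls Jump and sets a higher jump velocity when moving than when still; DisableMovement gates it and both move functions.
; JumpEnd only clears the JumpPressed flag.
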(event EventBeginPlay
  (Pawn|SpawnDefaultController))

(event Collision|EventActorBeginOverlap
  (params (OtherActor :type Actor%20Object%20Reference)))

(event EventTick
  (params (DeltaSeconds :type Float%20%28single-precision%29)))

(fn ConstructionScript)

(fn MoveForward
  (params (Axis_Value :type Float%20%28single-precision%29))
  (if (not (Variables|Default|GetDisableMovement))
    (Pawn|Input|AddControllerYawInput Axis_Value)
    (Pawn|Input|AddMovementInput (Math|Vector|MakeVector 1.0 0.0 0.0) Axis_Value false)))

(fn MoveRight
  (params (Axis_Value :type Float%20%28single-precision%29))
  (if (not (Variables|Default|GetDisableMovement))
    (Pawn|Input|AddMovementInput (Math|Vector|MakeVector 0.0 1.0 0.0) Axis_Value false)))

(fn JumpStart
  (bind _charactermovement (Variables|Character|GetCharacterMovement))
  (if (not (Variables|Default|GetDisableMovement))
    ;[1 1 1] Check if the character is currently moving
    (if (> (Math|Vector|VectorLength (Variables|/Script/Engine.MovementComponent|GetVelocity (Variables|Character|GetCharacterMovement))) 0.0)
      ;[1 1 1] Have the character Jump with a velocity dependent on whether the character is currently moving
      (Character|Jump)
      (Variables|/Script/Engine.CharacterMovementComponent|SetJumpZVelocity _charactermovement 2e+02)
      (Variables|Default|SetJumpPressed true)
      (else
        (Character|Jump)
        (Variables|/Script/Engine.CharacterMovementComponent|SetJumpZVelocity _charactermovement 1.8e+02)
        (Variables|Default|SetJumpPressed true)))))

(fn JumpEnd
  (Variables|Default|SetJumpPressed false))